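; Dungeon door Blueprint that opens on an event call with a camera shake, then hands the view back to the player.
; The opendoor event adds a camera shake source to the referenced camera's owner and starts the shake.
; A timeline lerps the door cube straight down.
; When it finishes, a short delay precedes a blend of the first player controller's view target to the passed-in Player.
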(event `open door`
  (params (player :type "Actor Object Reference"))
  (bind _returnvalue (`AddComponent|NODE_AddCameraShakeSourceComponent-0` :`self` (`ActorComponent.GetOwner` (`self.Camera`))))
  (`CameraShakeSourceComponent.StartCameraShake` :`self` _returnvalue :`InCameraShake` "/Game/Actors/MyShake.MyShake_C" :`Scale` 10.0)
  (bind (_direction _open_track) (`Timeline|open door t`)
    (:`Update`
      (`SceneComponent.K2_SetRelativeLocation` (`self.Cube`) (`KismetMathLibrary.VLerp` (0.0 0.0 0.0) (0.0 0.0 -800.0) _open_track) false false))
    (:`Finished`
      (`KismetSystemLibrary.Delay` 1.0)
      (`PlayerController.SetViewTargetWithBlend` (`GameplayStatics.GetPlayerController` 0) player 0.5 "VTBlend_Linear" 1.0 false))))

(fn `UserConstructionScript`)